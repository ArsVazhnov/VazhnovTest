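; Behavior tree task that makes an AI-controlled NPC destroy itself with sound and particle effects.
; On execute, it gets the pawn from the NPC AI controller and spawns the sound and emitter from that NPC's data asset at its location.
; It then destroys the pawn and finishes the task successfully.
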(event `self.ReceiveExecute`
  (params (OwnerActor :type "Actor Object Reference"))
  ;[1 1 1] Spawn FX for Npc from its Data Asset, then destroy Npc
  (bind _asbp_npc_aicontroller (cast `/Game/Blueprints/BP_NpcAIController` OwnerActor))
  (bind _returnvalue (`Controller.K2_GetPawn` _asbp_npc_aicontroller))
  (bind _asnpc (cast `Npc` _returnvalue))
  (`self.SpawnNpcFX` _asnpc)
  (`Actor.K2_DestroyActor` _returnvalue)
  (`self.FinishExecute` true))

(fn `SpawnNpcFX`
  (params (CurrentNpc :type "Npc Object Reference"))
  (bind _npcdata (`Npc.NpcData` CurrentNpc))
  (bind _returnvalue (`Actor.K2_GetActorLocation` (`local.CurrentNpc`)))
  (`GameplayStatics.SpawnSoundAtLocation` (`NpcData.NpcSFX` _npcdata) _returnvalue (struct) 1.0 1.0 0.0 null null)
  (`GameplayStatics.SpawnEmitterAtLocation` (`NpcData.NpcVFX` _npcdata) _returnvalue))